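; HUD class for the shooting game mode that creates the on-screen widget and shows the local player's HP, magazine and SH values.
; On BeginPlay it adds the widget, switches input to game-only and hides the cursor.
; It binds to BP_ShootingPlayerState dispatchers and pushes initial values, retrying on a short timer until that state exists.
; Update functions forward values to the widget; UpdateAmmo is defined but not bound here.
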(event `self.ReceiveBeginPlay`
  (bind _returnvalue (`GameplayStatics.GetPlayerController` 0))
  (bind _returnvalue_2 (`|CreateWidget` "/Game/Shooting/Widgets/Game/ShootingHudWidget.ShootingHudWidget_C"))
  (bind _output_get (set `self.HudWidget` _returnvalue_2))
  (`UserWidget.AddToViewport` _output_get 0)
  (`self.BindMyPlayerState`)
  (`WidgetBlueprintLibrary.SetInputMode_GameOnly` _returnvalue)
  (set `PlayerController.bShowMouseCursor` false _returnvalue))

(fn `BindMyPlayerState`
  (bind _asbp_shooting_player_state (cast `/Game/Shooting/GameMode/Game/BP_ShootingPlayerState` (`Controller.PlayerState` (`GameplayStatics.GetPlayerController` 0)))
    (:`then`
      (add `/Game/Shooting/GameMode/Game/BP_ShootingPlayerState.EventDispatcher_UpdateHp` _asbp_shooting_player_state (`|CreateDelegate` :!event `UpdateHp`))
      (`self.UpdateHp` (`/Game/Shooting/GameMode/Game/BP_ShootingPlayerState.CurHp` _asbp_shooting_player_state) (`/Game/Shooting/GameMode/Game/BP_ShootingPlayerState.MaxHp` _asbp_shooting_player_state))
      (add `/Game/Shooting/GameMode/Game/BP_ShootingPlayerState.EventDispatcher_UpdateMag` _asbp_shooting_player_state (`|CreateDelegate` :!event `UpdateMag`))
      (`self.UpdateMag` (`/Game/Shooting/GameMode/Game/BP_ShootingPlayerState.CurMag` _asbp_shooting_player_state))
      (add `/Game/Shooting/GameMode/Game/BP_ShootingPlayerState.EventDispatcher_UpdateSH` _asbp_shooting_player_state (`|CreateDelegate` :!event `UpdateSH`))
      (`self.UpdateSH` (`/Game/Shooting/GameMode/Game/BP_ShootingPlayerState.CurSH` _asbp_shooting_player_state) (`/Game/Shooting/GameMode/Game/BP_ShootingPlayerState.MaxSH` _asbp_shooting_player_state)))
    (:`CastFailed`
      (`KismetSystemLibrary.K2_SetTimer` null "BindMyPlayerState" 0.01))))

(fn `UpdateAmmo`
  (params (Ammo :type Integer))
  (`/Game/Shooting/Widgets/Game/ShootingHudWidget.SetAmmo` (`self.HudWidget`) Ammo))

(fn `UpdateHp`
  (params (CurHp :type "Float (double-precision)") (MaxHp :type "Float (double-precision)"))
  (`/Game/Shooting/Widgets/Game/ShootingHudWidget.SetHp` (`self.HudWidget`) CurHp MaxHp))

(fn `UpdateMag`
  (params (CurMag :type Integer))
  (`/Game/Shooting/Widgets/Game/ShootingHudWidget.SetMag` (`self.HudWidget`) CurMag))

(fn `UpdateSH`
  (params (CurSH :type "Float (double-precision)") (MaxSH :type "Float (double-precision)"))
  (`/Game/Shooting/Widgets/Game/ShootingHudWidget.SetSH` (`self.HudWidget`) CurSH MaxSH))

(fn `UserConstructionScript`)