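; HUD Blueprint for the shooting game mode that displays the player's health.
; On BeginPlay it creates the shooting HUD widget, adds it to the viewport and initializes it to full health.
; It binds to the HP update dispatcher on the first player's BP_ShootingPlayerState, retrying on a short timer until that cast succeeds.
; UPDateHP passes the current-to-max HP ratio to the widget.
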(event `self.ReceiveBeginPlay`
  (bind _returnvalue (`|CreateWidget` "/Game/Shooting/Widget/ShootingHudWidget.ShootingHudWidget_C"))
  (bind _output_get (set `self.HudWidget` _returnvalue))
  (`UserWidget.AddToViewport` _output_get 0)
  (`self.UPDateHP` 100.0 100.0)
  (`self.BindHP`))

(fn `BindHP`
  (bind _asbp_shooting_player_state (cast `/Game/Shooting/Gamemode/BP_ShootingPlayerState` (`Controller.PlayerState` (`GameplayStatics.GetPlayerController` 0)))
    (:`then`
      (add `/Game/Shooting/Gamemode/BP_ShootingPlayerState.UpdateHP_EventDispatcher` _asbp_shooting_player_state (`|CreateDelegate` :!event `UPDateHP`)))
    (:`CastFailed`
      (`KismetSystemLibrary.K2_SetTimer` null "BindHP" 0.1))))

(fn `UPDateHP`
  (params (CurHP :type "Float (double-precision)") (MaxHP :type "Float (double-precision)"))
  (`/Game/Shooting/Widget/ShootingHudWidget.Set HP` (`self.HudWidget`) (/ CurHP MaxHP)))

(fn `UserConstructionScript`)