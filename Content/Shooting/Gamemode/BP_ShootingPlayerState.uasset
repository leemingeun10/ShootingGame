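; Player state for the shooting game mode that tracks a player's HP and magazine count.
; HP starts at max on BeginPlay, and AddDamage subtracts from it without clamping.
; The CurHp RepNotify prints a debug message and broadcasts current and max HP through the UpdateHp dispatcher.
; AddMag increments CurMag and broadcasts UpdateMag directly.
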(event `self.ReceiveBeginPlay`
  (set `self.CurHp` (`self.MaxHp`)))

(fn `AddDamage`
  (params (Damage :type "Float (double-precision)"))
  (set `self.CurHp` (- (`self.CurHp`) Damage)))

(fn `AddMag`
  (bind _output_get (set `self.CurMag` (+ (`self.CurMag`) 1)))
  (`self.EventDispatcher_UpdateMag` _output_get))

(fn `OnRep_CurHp`
  (`KismetSystemLibrary.PrintString` (`KismetStringLibrary.Concat_StrStr` "OnRep_CurHp " ", HP : " (`KismetStringLibrary.Conv_DoubleToString` (`self.CurHp`))) true true (struct :`G` 0.66 :`B` 1.0 :`A` 1.0) 30.0)
  (`self.EventDispatcher_UpdateHp` (`self.CurHp`) (`self.MaxHp`)))

(fn `UserConstructionScript`)