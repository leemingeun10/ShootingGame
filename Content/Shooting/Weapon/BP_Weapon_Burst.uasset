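; Burst-fire weapon Blueprint that turns one trigger press into three timed calls to the parent's PlayAnim.
; EventTrigger resets a counter and starts a short looping timer by function name, ignoring releases and presses while that timer exists.
; The PlayAnim override runs the parent version, increments the counter and clears the timer after the third call.
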(fn `EventTrigger`
  (params (Press :type Boolean))
  (returns (Result :type Boolean))
  (if Press
    (if (not (`KismetSystemLibrary.K2_TimerExists` null "PlayAnim"))
      (set `self.Count` 0)
      (`KismetSystemLibrary.K2_SetTimer` null "PlayAnim" 0.1 true)
      (return false))))

(fn `PlayAnim`
  (`parent.PlayAnim`)
  (bind _output_get (set `self.Count` (+ (`self.Count`) 1)))
  (if (>= _output_get 3)
    (`KismetSystemLibrary.K2_ClearTimer` null "PlayAnim")))

(fn `UserConstructionScript`
  (`parent.UserConstructionScript`))