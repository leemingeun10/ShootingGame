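; Actor component that manages timed buffs on its owner in the shooting game, currently handling an Invincible buff.
; AddBuff looks up a DT_Buff row, stores it with an elapsed time and applies its effect by type.
; Each Tick advances timers, then removes expired buffs one at a time, rescanning until none remain.
; Invincibility sets a queryable flag and attaches a Niagara effect to the Character's mesh, both cleared on removal.
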(event `self.ReceiveTick`
  (params (DeltaSeconds :type "Float (single-precision)"))
  (`self.UpdateBuffTick` DeltaSeconds))

(fn `AddBuff`
  (params (RowName :type Name))
  (bind _returnvalue (`|GetDataTableRow` "/Game/Shooting/Buff/DT_Buff.DT_Buff" RowName)
    (:`then`
      (`KismetArrayLibrary.Array_Add` (`self.Buffs`) (make `/Game/Shooting/Buff/ST_BuffRef` _returnvalue))
      (`self.EventApplyBuff` _returnvalue))))

(fn `EventApplyBuff`
  (params (Buff :type "/Game/Shooting/Buff/ST_Buff Structure"))
  (switch `/Game/Shooting/Buff/EN_BuffType` (`.BuffType_10_01A03F0645091D77A335F882F6CE0661` (break `/Game/Shooting/Buff/ST_Buff` Buff))
    (:`NewEnumerator1`
      (set `self.Invincible` true)
      (bind _ascharacter (cast `Character` (`self.GetOwner`)))
      (bind _returnvalue (`NiagaraFunctionLibrary.SpawnSystemAttached` "/Game/Basic_VFX/Niagara/NS_Basic_9.NS_Basic_9" (`Character.Mesh` _ascharacter) "None" (0.0 0.0 30.0) (struct) "KeepRelativeOffset"))
      (set `self.InvincibleEffect` _returnvalue))))

(fn `EventRemoveBuff`
  (params (Buff :type "/Game/Shooting/Buff/ST_Buff Structure"))
  (switch `/Game/Shooting/Buff/EN_BuffType` (`.BuffType_10_01A03F0645091D77A335F882F6CE0661` (break `/Game/Shooting/Buff/ST_Buff` Buff))
    (:`NewEnumerator1`
      (set `self.Invincible` false)
      (bind _invincibleeffect (`self.InvincibleEffect`)
        (:`then`
          (`self.K2_DestroyComponent` _invincibleeffect))
        (:`else`)))))

(fn `IsInvincible`
  (returns (IsInvincible :type Boolean))
  (return (`self.Invincible`)))

(fn `UpdateBuffTick`
  (params (DeltaSeconds :type "Float (double-precision)"))
  (`|ExecutionSequence`
    (:`then_0`
      (`self.UpdateBuffTime` DeltaSeconds))
    (:`then_1`
      (bind _iscomplated (`self.UpdateBuffTimeOver` :!label _label))
      (if (not _iscomplated)
        (goto _label)))))

(fn `UpdateBuffTime`
  (params (DeltaSeconds :type "Float (double-precision)"))
  (for (_ _array_index) (`self.Buffs`)
    (bind _output (`|GetArrayItem` (`self.Buffs`) _array_index))
    (setmembers `/Game/Shooting/Buff/ST_BuffRef` :`StructRef` _output :`CurDuration` (+ (`.CurDuration_5_271C8CE54D8D8A1E21DB4F8D6C35F6E7` (break `/Game/Shooting/Buff/ST_BuffRef` _output)) (`local.DeltaSeconds`)))))

(fn `UpdateBuffTimeOver`
  (returns (IsComplated :type Boolean))
  (for (_array_element _array_index) (`self.Buffs`)
    (bind (_buffdata _curduration) (break `/Game/Shooting/Buff/ST_BuffRef` _array_element))
    (if (<= (`.Duration_8_B680ABE747FBDA3E7D082FB31FC3EEA2` (break `/Game/Shooting/Buff/ST_Buff` _buffdata)) _curduration)
      (`self.EventRemoveBuff` (`.BuffData_3_DE2E72704A58A6C530D3589210FA7A0D` (break `/Game/Shooting/Buff/ST_BuffRef` _array_element)))
      (`KismetArrayLibrary.Array_Remove` (`self.Buffs`) _array_index)
      (return false)))
  (return true))