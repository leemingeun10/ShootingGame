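; BP_actorSpawner is a trigger actor that spawns a BP_NetBall when a BP_ShootingCharacter overlaps its Cube component.
; The overlap is handled only with authority, then passes through the ReqSpawn and ResponseSpawn events to the SpawnActor function.
; SpawnActor places each ball at the world transform of the Arrow component.
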(event `ReqSpawn`
  (`self.ResponseSpawn`))

(event `self.Cube.OnComponentBeginOverlap`
  (params (OverlappedComponent :type "PrimitiveComponent Object Reference") (OtherActor :type "Actor Object Reference") (OtherComp :type "PrimitiveComponent Object Reference") (OtherBodyIndex :type Integer) (bFromSweep :type Boolean) (SweepResult :type "HitResult Structure (by ref)"))
  (`/Engine/EditorBlueprintResources/ActorMacros.Switch Has Authority`
    (:`Authority`
      (cast `/Game/Shooting/Gamemode/BP_ShootingCharacter` OtherActor)
      (`self.ReqSpawn`))))

(event `ResponseSpawn`
  (`self.SpawnActor`))

(fn `SpawnActor`
  (`|SpawnActorFromClass` "/Game/Shooting/BluePrints/BP_NetBall.BP_NetBall_C" (`SceneComponent.K2_GetComponentToWorld` (`self.Arrow`)) "Undefined" "MultiplyWithRoot" null null))

(fn `UserConstructionScript`)