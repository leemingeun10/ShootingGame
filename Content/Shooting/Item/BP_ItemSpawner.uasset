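; BP_ItemSpawner is an actor that keeps a random item from its Items list spawned at its location.
; On BeginPlay, the authority spawns a random class at the spawner's transform and binds to that actor's OnDestroyed event.
; A failed spawn retries on a five-second timer, and EventItemDestroy uses the same delay to respawn after the item is destroyed.
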(event `self.ReceiveBeginPlay`
  (`self.DoRandomItemSpawn`))

(fn `DoRandomItemSpawn`
  (`/Engine/EditorBlueprintResources/ActorMacros.Switch Has Authority`
    (:`Authority`
      (bind _returnvalue (`|SpawnActorFromClass` (`KismetArrayLibrary.Array_Random` (`self.Items`)) (`self.GetTransform`) "Undefined" "MultiplyWithRoot" null null))
      (`/Engine/EditorBlueprintResources/StandardMacros.IsValid` _returnvalue
        (:`Is Valid`
          (add `self.OnDestroyed` _returnvalue (`|CreateDelegate` :!event `EventItemDestroy`)))
        (:`Is Not Valid`
          (`KismetSystemLibrary.K2_SetTimer` null "DoRandomItemSpawn" 5.0))))))

(fn `EventItemDestroy`
  (params (DestroyedActor :type "Actor Object Reference"))
  (`KismetSystemLibrary.K2_SetTimer` null "DoRandomItemSpawn" 5.0))

(fn `UserConstructionScript`)